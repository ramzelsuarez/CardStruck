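; BP_CatGirl is the player-controlled cat girl character, with movement, look, jump and two kick attacks.
; On possession it adds its Enhanced Input mapping context, then moves relative to control yaw, with Left Shift toggling half and full speed.
; Left and right mouse play super and simple kick montages and record the type in KickST.
; CollisionON and CollisionOFF events switch the FootCapsule's collision, with their callers outside this graph.
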(event Custom|CollisionON
  (Collision|SetCollisionEnabled (Variables|Default|GetFoot_Capsule) "QueryAndPhysics"))

(event Custom|CollisionOFF
  (Collision|SetCollisionEnabled (Variables|Default|GetFoot_Capsule) "NoCollision"))

(event Input|EnhancedActionEvents|EnhancedInputActionIA_Jump
  (params (ActionValue :type Boolean) (ElapsedSeconds :type Float%20%28double-precision%29) (TriggeredSeconds :type Float%20%28double-precision%29) (InputAction :type Input%20Action%20Object%20Reference :default "/Game/Character/ProjectMappings/IA_Jump.IA_Jump"))
  (Character|Jump))

(event Input|EnhancedActionEvents|EnhancedInputActionIA_Turn
  (params (ActionValue :type Float%20%28double-precision%29) (ElapsedSeconds :type Float%20%28double-precision%29) (TriggeredSeconds :type Float%20%28double-precision%29) (InputAction :type Input%20Action%20Object%20Reference :default "/Game/Character/ProjectMappings/IA_Turn.IA_Turn"))
  (Pawn|Input|AddControllerYawInput ActionValue))

(event Input|EnhancedActionEvents|EnhancedInputActionIA_LookUp
  (params (ActionValue :type Float%20%28double-precision%29) (ElapsedSeconds :type Float%20%28double-precision%29) (TriggeredSeconds :type Float%20%28double-precision%29) (InputAction :type Input%20Action%20Object%20Reference :default "/Game/Character/ProjectMappings/IA_LookUp.IA_LookUp"))
  (Pawn|Input|AddControllerPitchInput ActionValue))

(event Input|EnhancedActionEvents|EnhancedInputActionIA_WS
  (params (ActionValue :type Float%20%28double-precision%29) (ElapsedSeconds :type Float%20%28double-precision%29) (TriggeredSeconds :type Float%20%28double-precision%29) (InputAction :type Input%20Action%20Object%20Reference :default "/Game/Character/ProjectMappings/IA_WS.IA_WS"))
  (Pawn|Input|AddMovementInput (Math|Vector|GetForwardVector (Math|Rotator|MakeRotator 0.0 0.0 (.yaw (Pawn|GetControlRotation :!class /Script/Engine.Pawn)))) (* ActionValue (Variables|Default|GetSpeed)) false))

(event Input|EnhancedActionEvents|EnhancedInputActionIA_AD
  (params (ActionValue :type Float%20%28double-precision%29) (ElapsedSeconds :type Float%20%28double-precision%29) (TriggeredSeconds :type Float%20%28double-precision%29) (InputAction :type Input%20Action%20Object%20Reference :default "/Game/Character/ProjectMappings/IA_AD.IA_AD"))
  (Pawn|Input|AddMovementInput (Math|Vector|GetRightVector (Math|Rotator|MakeRotator 0.0 0.0 (.yaw (Pawn|GetControlRotation :!class /Script/Engine.Pawn)))) (* ActionValue (Variables|Default|GetSpeed)) false))

(event Input|EnhancedActionEvents|EnhancedInputActionIA_MouseL
  (params (ActionValue :type Boolean) (ElapsedSeconds :type Float%20%28double-precision%29) (TriggeredSeconds :type Float%20%28double-precision%29) (InputAction :type Input%20Action%20Object%20Reference :default "/Game/Character/ProjectMappings/IA_MouseL.IA_MouseL"))
  (Animation|Montage|PlayMontage (Variables|Character|GetMesh) "/Game/Character/AnimMon_CatGirlSUPERKICK.AnimMon_CatGirlSUPERKICK"
    (:then
      (Variables|Default|SetKick_ST 1))))

(event Input|EnhancedActionEvents|EnhancedInputActionIA_MouseR
  (params (ActionValue :type Boolean) (ElapsedSeconds :type Float%20%28double-precision%29) (TriggeredSeconds :type Float%20%28double-precision%29) (InputAction :type Input%20Action%20Object%20Reference :default "/Game/Character/ProjectMappings/IA_MouseR.IA_MouseR"))
  (Animation|Montage|PlayMontage (Variables|Character|GetMesh) "/Game/Character/AnimMon_SIMPLEKICK.AnimMon_SIMPLEKICK"
    (:then
      (Variables|Default|SetKick_ST 0))))

(event EventPossessed
  (params (NewController :type Controller%20Object%20Reference))
  (bind _asplayer_controller (Utilities|Casting|CastToPlayerController NewController))
  (Input|AddMappingContext (PlayerController|LocalPlayerSubsystems|GetEnhancedInputLocalPlayerSubsystem _asplayer_controller) "/Game/Character/ProjectMappings/IMC_CatGirl.IMC_CatGirl" 0 "(bIgnoreAllPressedKeysUntilRelease=True,bForceImmediately=False,bNotifyUserSettings=False)"))

(event Input|KeyboardEvents|LeftShift
  (params (Key :type Key%20Structure :default "None"))
  (:Pressed
    (Utilities|FlowControl|FlipFlop
      (:A
        (Variables|Default|SetSpeed 0.5))
      (:B
        (Variables|Default|SetSpeed 1.0)))))

(fn ConstructionScript)